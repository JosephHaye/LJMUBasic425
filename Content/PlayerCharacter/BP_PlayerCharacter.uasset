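; Player character Blueprint with intro music, a launch-velocity debug print and unfinished weapon switching.
; BeginPlay plays the music at the actor's location, and the Throw event holds HasThrown true for three seconds.
; Q and E both only decrement CurrentWeapon under index checks, then cast the Inventory child actor to BP_AR or BP_GL without further action.
; The logic that spawns both weapons into a WeaponArray is disconnected and never runs.
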(event EventBeginPlay
  ;[1 1 1] Plays sound at location
  (Audio|PlaySoundatLocation "/Game/Assets/Sounds/Music/Music_Intro.Music_Intro" (Transformation|GetActorLocation) "0, 0, 0" 1.0 1.0 0.0 0 0 0))

(event EventThrow
  ;[1 1 1] Throw
  (Variables|Default|SetHasThrown true)
  (Utilities|FlowControl|Delay 3.0)
  (Variables|Default|SetHasThrown false))

(event EventTick
  (params (DeltaSeconds :type Float%20%28single-precision%29))
  ;[1 1 1] Debug For current weapon
)

(event EventOnLaunched
  (params (LaunchVelocity :type Vector :default "0, 0, 0") (bXYOverride :type Boolean) (bZOverride :type Boolean))
  ;[1 1 1] Debug Code
  (Development|PrintString (Utilities|String|BuildString(Vector) "" "Launched" LaunchVelocity)))

(event Input|KeyboardEvents|Q
  (params (Key :type Key%20Structure :default "None"))
  ;[1 1 1] Change weapon
  (:Pressed
    (if (< (Variables|Default|GetCurrentWeapon) 0)
      (Variables|Default|SetCurrentWeapon (- (Variables|Default|GetCurrentWeapon) 1))
      (Utilities|Casting|CastToBP_AR (Variables|/Script/Engine.ChildActorComponent|GetChildActor (Variables|Default|GetInventory))))))

(event Input|KeyboardEvents|E
  (params (Key :type Key%20Structure :default "None"))
  ;[1 1 1] Change weapon
  (:Pressed
    (if (< (Variables|Default|GetCurrentWeapon) 1)
      (Variables|Default|SetCurrentWeapon (- (Variables|Default|GetCurrentWeapon) 1))
      (Utilities|Casting|CastToBP_GL (Variables|/Script/Engine.ChildActorComponent|GetChildActor (Variables|Default|GetInventory))))))

(fn ConstructionScript)